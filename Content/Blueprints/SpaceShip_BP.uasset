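; Player ship for a meteorite shooter on the X-Z plane, which spawns flashing with collision off until the flash timeline finishes.
; Each tick it turns toward the Touch1 hit point, moves with eased input-driven drift and wraps past play-area bounds.
; Fire launches rate-limited projectiles along its local up axis.
; Meteorite overlap destroys it, spawning an explosion and asking the game mode to try a respawn.
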(event OnComponentBeginOverlap(ShipSprite)
  (params (OverlappedComponent :type Primitive%20Component%20Object%20Reference) (OtherActor :type Actor%20Object%20Reference) (OtherComp :type Primitive%20Component%20Object%20Reference) (OtherBodyIndex :type Integer) (bFromSweep :type Boolean) (SweepResult :type Hit%20Result%20Structure%20%28by%20ref%29))
  (Utilities|Casting|CastToMeteorite_BP OtherActor)
  (Actor|DestroyActor))

(event Custom|OnDestroyed_Event
  (params (DestroyedActor :type Actor%20Object%20Reference))
  ;[1 1 1] Comment
  (Class|ActionsInterfaceBP|TrytoSpawnPlayer(Message) (Game|GetGameMode))
  (Game|SpawnActorfromClass "/Game/Blueprints/Explosion_BP.Explosion_BP_C" (Math|Conversions|ToTransform(Vector) (Transformation|GetActorLocation)) "Undefined" 0 0))

(event EventBeginPlay
  (bind _ship_sprite (Variables|Default|GetShip%20Sprite))
  ;[1 1 1] Comment
  (Collision|SetCollisionEnabled (Variables|Default|GetShip%20Sprite) "NoCollision")
  (Game|BindEventtoOnDestroyed (delegate Custom|OnDestroyed_Event))
  (Input|EnableInput (Game|GetPlayerController 0))
  (bind _value (Timeline|Flashing%20Timeline Play)
    (:Update
      (Sprite|SetSpriteColor _ship_sprite (Utilities|Struct|MakeLinearColor 1.0 1.0 1.0 _value)))
    (:Finished
      (Collision|SetCollisionEnabled _ship_sprite "QueryAndPhysics"))))

(event EventTick
  (params (DeltaSeconds :type Float%20%28single-precision%29))
  (|RotateShipWithMouse)
  (|MoveShip)
  (|LimitsDirection))

(event Input|ActionEvents|InputActionFireAction
  (params (Key :type Key%20Structure :default "None"))
  (:Pressed
    (|FireProjectile)))

(fn ConstructionScript)